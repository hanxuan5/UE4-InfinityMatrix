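; Player-fired projectile that destroys enemies and awards score.
; Each tick it moves along world X with a swept offset, at a speed set through SetProjectileSpeed (which doubles the input), and expires after a short lifetime.
; When its sphere overlaps a BP_Enemy, it updates the stored Player's score and score bar, then destroys both the enemy and itself.
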(event `self.ReceiveTick`
  (params (DeltaSeconds :type "Float (single-precision)"))
  (`self.K2_AddActorWorldOffset` (`KismetMathLibrary.MakeVector` (* DeltaSeconds (`self.Forward`))) true)
  (if (> (`self.GetGameTimeSinceCreation`) 2.0)
    (`self.K2_DestroyActor`)))

(event `self.Sphere1.OnComponentBeginOverlap`
  (params (OverlappedComponent :type "PrimitiveComponent Object Reference") (OtherActor :type "Actor Object Reference") (OtherComp :type "PrimitiveComponent Object Reference") (OtherBodyIndex :type Integer) (bFromSweep :type Boolean) (SweepResult :type "HitResult Structure (by ref)"))
  (bind _player (`self.Player`))
  (bind _asbp_enemy (cast `/Game/InfiniteMatrix/Blueprints/BP_Enemy` OtherActor))
  (`/Game/InfiniteMatrix/Blueprints/BP_Player.UpdateScore` _player 10)
  (`/Game/InfiniteMatrix/Blueprints/BP_Player.UpdateScoreBar` _player)
  (`self.K2_DestroyActor` _asbp_enemy)
  (`self.K2_DestroyActor`))

(fn `SetProjectilePlayer`
  (params (player :type "/Game/InfiniteMatrix/Blueprints/BP_Player Object Reference"))
  (set `self.Player` player))

(fn `SetProjectileSpeed`
  (params (Input :type "Float (double-precision)"))
  (set `self.Forward` (* Input 2.0)))

(fn `UserConstructionScript`)