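; Spawner actor that builds an endless chain of BP_Tunnel segments, with randomly placed enemies and healthpacks.
; On BeginPlay it destroys existing tunnels, healthpacks and enemies through nested loops, then spawns a few starting segments from the player's location.
; Each new segment attaches at the newest tunnel's SpawnPoint, gets a randomized wall and a back-reference to the spawner for further spawning.
; Enemies and healthpacks each have a one-in-five chance per segment, at a random offset.
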(event `self.ReceiveBeginPlay`
  (`self.Spawn Initial Tunnels`))

(fn `Spawn Enemy`
  (params (Location :type "Vector Structure"))
  (if (== (select `int` (`KismetMathLibrary.RandomIntegerInRange` 0 4) :`0` 0 :`1` 1 :`2` 2 :`3` 3 :`4` 4) 0)
    (`|SpawnActorFromClass` "/Game/InfiniteMatrix/Blueprints/BP_Enemy.BP_Enemy_C" (`KismetMathLibrary.MakeTransform` (+ Location (`KismetMathLibrary.MakeVector` (`KismetMathLibrary.RandomFloatInRange` 500.0 800.0) (`KismetMathLibrary.RandomFloatInRange` -300.0 300.0) (`KismetMathLibrary.RandomFloatInRange` -300.0 300.0)))) "Undefined" "OverrideRootScale" null null)))

(fn `Spawn Healthpack`
  (params (Location :type "Vector Structure"))
  (if (== (select `int` (`KismetMathLibrary.RandomIntegerInRange` 0 4) :`0` 0 :`1` 1 :`2` 2 :`3` 3 :`4` 4) 0)
    (`|SpawnActorFromClass` "/Game/InfiniteMatrix/Blueprints/BP_Healthpack.BP_Healthpack_C" (`KismetMathLibrary.MakeTransform` (+ Location (`KismetMathLibrary.MakeVector` (`KismetMathLibrary.RandomFloatInRange` 500.0 800.0) (`KismetMathLibrary.RandomFloatInRange` -300.0 300.0) (`KismetMathLibrary.RandomFloatInRange` -300.0 300.0)))) "Undefined" "OverrideRootScale" null null)))

(fn `Spawn Initial Tunnels`
  (`|ExecutionSequence`
    (:`then_0`
      (bind _outactors (`GameplayStatics.GetAllActorsOfClass` "/Game/InfiniteMatrix/Blueprints/BP_Tunnel.BP_Tunnel_C"))
      (for _array_element _outactors
        (`self.K2_DestroyActor` _array_element)
        (bind _outactors_2 (`GameplayStatics.GetAllActorsOfClass` "/Game/InfiniteMatrix/Blueprints/BP_Healthpack.BP_Healthpack_C"))
        (for _array_element_2 _outactors_2
          (`self.K2_DestroyActor` _array_element_2)
          (bind _outactors_3 (`GameplayStatics.GetAllActorsOfClass` "/Game/InfiniteMatrix/Blueprints/BP_Enemy.BP_Enemy_C"))
          (for _array_element_3 _outactors_3
            (`self.K2_DestroyActor` _array_element_3)))))
    (:`then_1`
      (for _ (range 3)
        (`/Engine/EditorBlueprintResources/StandardMacros.IsValid` (`self.Newest Tunnel`)
          (:`Is Valid`
            (`self.SpawnTunnelAtSpawnPoint`))
          (:`Is Not Valid`
            (`self.Spawn Tunnel` (`self.K2_GetActorLocation` (`GameplayStatics.GetPlayerPawn` 0)))))))))

(fn `Spawn Tunnel`
  (params (SpawnLocation :type "Vector Structure"))
  (`self.Spawn Enemy` SpawnLocation)
  (`self.Spawn Healthpack` SpawnLocation)
  (bind _returnvalue (`|SpawnActorFromClass` "/Game/InfiniteMatrix/Blueprints/BP_Tunnel.BP_Tunnel_C" (`KismetMathLibrary.MakeTransform` SpawnLocation) "Undefined" "OverrideRootScale" null null))
  (bind _output_get (set `self.Newest Tunnel` _returnvalue))
  (set `/Game/InfiniteMatrix/Blueprints/BP_Tunnel.TunnelSpawner` self _output_get)
  (`/Game/InfiniteMatrix/Blueprints/BP_Tunnel.RandomizeWall` _output_get))

(fn `SpawnTunnelAtSpawnPoint`
  (`self.Spawn Tunnel` (`SceneComponent.K2_GetComponentLocation` (`/Game/InfiniteMatrix/Blueprints/BP_Tunnel.SpawnPoint` (`self.Newest Tunnel`)))))

(fn `UserConstructionScript`)