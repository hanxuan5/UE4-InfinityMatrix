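; BP_Healthpack is a pickup that adds health to BP_Player when the player overlaps its collision component, then destroys itself.
; Projectiles that hit it are destroyed along with the pack, and contact with an enemy destroys only the pack.
; Tick also destroys the pack once its X position falls below the player pawn's, removing packs the player has passed.
; The CreateHealthpack function is an empty stub.
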(event `self.ReceiveTick`
  (params (DeltaSeconds :type "Float (single-precision)"))
  (bind _returnvalue_x (`KismetMathLibrary.BreakVector` (`self.K2_GetActorLocation`)))
  (bind _returnvalue_x_2 (`KismetMathLibrary.BreakVector` (`self.K2_GetActorLocation` (`GameplayStatics.GetPlayerPawn` 0))))
  (if (< _returnvalue_x _returnvalue_x_2)
    (`self.K2_DestroyActor`)))

(event `self.HealthpackCollision.OnComponentBeginOverlap`
  (params (OverlappedComponent :type "PrimitiveComponent Object Reference") (OtherActor :type "Actor Object Reference") (OtherComp :type "PrimitiveComponent Object Reference") (OtherBodyIndex :type Integer) (bFromSweep :type Boolean) (SweepResult :type "HitResult Structure (by ref)"))
  (bind _asbp_player (cast `/Game/InfiniteMatrix/Blueprints/BP_Player` OtherActor)
    (:`then`
      (`/Game/InfiniteMatrix/Blueprints/BP_Player.AddHealth` _asbp_player)
      (`self.K2_DestroyActor` :!label _label))
    (:`CastFailed`
      (bind _asbp_projectile (cast `/Game/InfiniteMatrix/Blueprints/BP_projectile` OtherActor)
        (:`then`
          (`self.K2_DestroyActor` _asbp_projectile)
          (goto _label))
        (:`CastFailed`
          (cast `/Game/InfiniteMatrix/Blueprints/BP_Enemy` OtherActor)
          (`self.K2_DestroyActor`))))))

(fn `CreateHealthpack`)

(fn `UserConstructionScript`)